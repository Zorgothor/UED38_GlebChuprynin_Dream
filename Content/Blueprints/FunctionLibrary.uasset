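; Blueprint function library that holds a single helper, RngVectorScale, for randomly scaling a vector.
; It multiplies X, Y and Z each by its own random float drawn between the supplied min and max, so the scaling can be non-uniform.
; The scaled components return as three separate floats rather than a combined vector.
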(fn RngVectorScale
  (params (InVector :type Vector) (InMax :type Float%20%28double-precision%29) (InMin :type Float%20%28double-precision%29))
  (return (Math|Vector|MakeVector (* (Math|Random|RandomFloatinRange InMin InMax) (.x InVector)) (* (Math|Random|RandomFloatinRange InMin InMax) (.y InVector)) (* (Math|Random|RandomFloatinRange InMin InMax) (.z InVector)))))