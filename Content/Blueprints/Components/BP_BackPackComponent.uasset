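; Backpack component for a BP_CharacterBase owner that stores quest items and reserve ammo per weapon name; consumable item functions are empty stubs.
; UpdateAmmoByName adds or subtracts reserve ammo, clamped between zero and the equipped weapon's max rounds, whichever weapon is named.
; Adding ammo when both reserve and equipped weapon are empty also changes that weapon's state.
; Tick prints all reserve counts on screen for debugging.
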(event EventBeginPlay)

(event EventTick
  (params (DeltaSeconds :type Float%20%28single-precision%29))
  (CallFunction|DebugAmmo))

(fn AddQuestItem
  (params (InItemName :type Name))
  (Utilities|Set|Add (Variables|Inventory|GetQuestItems) InItemName))

(fn RemoveQuestItem
  (params (InItemName :type Name))
  (bind _returnvalue (Utilities|Set|Remove (Variables|Inventory|GetQuestItems) InItemName))
  (return _returnvalue))

(fn AddConsumerableItem)

(fn RemoveConsumerableItem
  (return))

(fn UpdateAmmobyName
  (params (InAmmo :type Integer) (InIncreased :type Boolean) (InWeaponName :type Name))
  (bind _availableweapons (Variables|Inventory|GetAvailableWeapons))
  (bind (_value _returnvalue) (Utilities|Map|Find _availableweapons InWeaponName))
  (bind _asbp_character_base (Utilities|Casting|CastToBP_CharacterBase (Components|GetOwner)))
  (bind _currentweapon (Variables|/Game/Blueprints/Character/BP_CharacterBase.BP_CharacterBase_C|GetCurrentWeapon _asbp_character_base)
    (:then
      (LocalVariables|SetL_CurrentWeapon _currentweapon)
      (if _returnvalue
        (LocalVariables|SetL_AmmoInBackpackCurrent _value)
        (Utilities|FlowControl|Sequence
          (:then_0
            (if InIncreased
              (Utilities|FlowControl|Sequence
                (:then_0
                  (if (<= (LocalVariables|GetL_AmmoInBackpackCurrent) 0)
                    (if (<= (Variables|/Game/Blueprints/Weapons/BP_BaseWeapon.BP_BaseWeapon_C|GetRoundsCurrent (LocalVariables|GetL_CurrentWeapon)) 0)
                      (Variables|/Game/Blueprints/Weapons/BP_BaseWeapon.BP_BaseWeapon_C|SetWeaponState (LocalVariables|GetL_CurrentWeapon) "NewEnumerator2"))))
                (:then_1
                  (bind _output_get (LocalVariables|SetL_Current (+ (LocalVariables|GetL_AmmoInBackpackCurrent) InAmmo)))
                  (if (< _output_get (Utilities|Struct|BreakSTRUCT_WeaponStats (Variables|/Game/Blueprints/Weapons/BP_BaseWeapon.BP_BaseWeapon_C|GetWeaponStats (LocalVariables|GetL_CurrentWeapon))))
                    (LocalVariables|SetL_AmmoInBackpackCurrent (LocalVariables|GetL_Current))
                    (LocalVariables|SetL_Current (Utilities|Struct|BreakSTRUCT_WeaponStats (Variables|/Game/Blueprints/Weapons/BP_BaseWeapon.BP_BaseWeapon_C|GetWeaponStats (LocalVariables|GetL_CurrentWeapon))))
                    (else
                      (LocalVariables|SetL_AmmoInBackpackCurrent (Utilities|Struct|BreakSTRUCT_WeaponStats (Variables|/Game/Blueprints/Weapons/BP_BaseWeapon.BP_BaseWeapon_C|GetWeaponStats (LocalVariables|GetL_CurrentWeapon))))))))
              (else
                (LocalVariables|SetL_Current (- (LocalVariables|GetL_AmmoInBackpackCurrent) InAmmo))
                (if (> (LocalVariables|GetL_Current) 0)
                  (LocalVariables|SetL_AmmoInBackpackCurrent (LocalVariables|GetL_Current))
                  (else
                    (LocalVariables|SetL_AmmoInBackpackCurrent 0)
                    (LocalVariables|SetL_Current (+ (LocalVariables|GetL_Current) (Utilities|Struct|BreakSTRUCT_WeaponStats (Variables|/Game/Blueprints/Weapons/BP_BaseWeapon.BP_BaseWeapon_C|GetWeaponStats (LocalVariables|GetL_CurrentWeapon))))))))))
          (:then_1
            (Utilities|Map|Add (Variables|Inventory|GetAvailableWeapons) InWeaponName (LocalVariables|GetL_AmmoInBackpackCurrent)))
          (:then_2
            (return (LocalVariables|GetL_Current))))
        (else
          (return 0))))
    (:else)))

(fn DebugAmmo
  (bind _values (Utilities|Map|Values (Variables|Inventory|GetAvailableWeapons)))
  (for _array_element _values
    (LocalVariables|SetL_String (Utilities|String|Append (LocalVariables|GetL_String) " | " (Utilities|String|ToString(Integer) _array_element))))
  (Development|PrintString (LocalVariables|GetL_String) true false "(R=0.000000,G=0.660000,B=1.000000,A=1.000000)" 0.0))