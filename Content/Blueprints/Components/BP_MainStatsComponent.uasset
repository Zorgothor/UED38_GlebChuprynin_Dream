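; Stats component that tracks a character's HP, EP shield, Fury and death state, plus Fury-based leveling.
; BeginPlay loads a DT_AllStats row by name to set walk speeds and starting values, which the player character instead restores from the save game when continuing.
; Damage, heal, shield and Fury functions broadcast changes through dispatchers.
; Total Fury is checked against DT_Leveling thresholds to award level points, which sync with W_SkillTree when spent.
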(event EventBeginPlay
  (CallFunction|ConfigureStats)
  (CallFunction|ConfigureNextLevelInfo)
  (Variables|Default|SetIsConfigSuccess true))

(event EventTick
  (params (DeltaSeconds :type Float%20%28single-precision%29)))

(fn ConfigureStats
  (if (!= (Variables|Default|GetCurrentName) "")
    (bind _returnvalue (Utilities|GetDataTableRow "/Game/Data/DT_AllStats.DT_AllStats" (Variables|Default|GetCurrentName))
      (:then
        (Variables|Default|SetMainStatsStructure _returnvalue)
        (Utilities|FlowControl|Sequence
          (:then_0
            (Config|ConfigureMovement))
          (:then_1
            (CallFunction|ConfigureHealthandEPandFury))))
      (:RowNotFound
        (Development|PrintString "Invalid DT Name!" false true "(R=1.000000,G=0.012401,B=0.000000,A=1.000000)")))
    (else
      (Development|PrintString "Invalid Name!" false true "(R=1.000000,G=0.012401,B=0.000000,A=1.000000)"))))

(fn ReceiveDamage
  (params (InDamage :type Float%20%28double-precision%29) (InDamageType :type ENUM_DamageType%20Enum :default "NewEnumerator0") (InCauser :type Actor%20Object%20Reference))
  (if (not (Variables|Default|GetIsDead))
    (bind _output_get (Variables|Default|SetCurrentHP (Math|Float|Truncate (- (Variables|Default|GetCurrentHP) InDamage))))
    (if (> _output_get 0)
      (Variables|Default|SetIsDead false)
      (else
        (Variables|Default|SetCurrentHP 0)
        (Variables|Default|SetIsDead true)))
    (Default|CallOnStatsUpdated (Variables|Default|GetCurrentHP) (Variables|Default|GetCurrentEP) (Variables|Default|GetIsDead) false (Variables|Default|GetCurrentFury))
    (if (Variables|Default|GetIsDead)
      (Default|CallOnDead)
      (else
        (Default|CallOnDamageRecieved InDamage InDamageType InCauser)))))

(fn HealUp
  (params (InToMaximum :type Boolean) (InAddHP :type Integer))
  (if InToMaximum
    (Variables|Default|SetCurrentHP (.MaxHP (Utilities|Struct|BreakSTRUCT_MainStats (Variables|Default|GetMainStatsStructure))))
    (else
      (Variables|Default|SetCurrentHP (Math|Integer|Min(Integer) (+ (Variables|Default|GetCurrentHP) InAddHP) (.MaxHP (Utilities|Struct|BreakSTRUCT_MainStats (Variables|Default|GetMainStatsStructure)))))))
  (Default|CallOnStatsUpdated (Variables|Default|GetCurrentHP) (Variables|Default|GetCurrentEP) (Variables|Default|GetIsDead) false (Variables|Default|GetCurrentFury)))

(fn ShieldUP
  (params (InToMaximum :type Boolean) (InAddEP :type Integer))
  (if InToMaximum
    (Variables|Default|SetCurrentEP (.MaxHP (Utilities|Struct|BreakSTRUCT_MainStats (Variables|Default|GetMainStatsStructure))))
    (else
      (Variables|Default|SetCurrentEP (Math|Integer|Min(Integer) (+ InAddEP (Variables|Default|GetCurrentEP)) (.MaxHP (Utilities|Struct|BreakSTRUCT_MainStats (Variables|Default|GetMainStatsStructure)))))))
  (Default|CallOnStatsUpdated (Variables|Default|GetCurrentHP) (Variables|Default|GetCurrentEP) (Variables|Default|GetIsDead) false (Variables|Default|GetCurrentFury)))

(fn CheckHP
  (return (== (Variables|Default|GetCurrentHP) (.MaxHP (Utilities|Struct|BreakSTRUCT_MainStats (Variables|Default|GetMainStatsStructure))))))

(fn CheckEP
  (return (== (Variables|Default|GetCurrentEP) (.MaxEP (Utilities|Struct|BreakSTRUCT_MainStats (Variables|Default|GetMainStatsStructure))))))

(fn ConfigureMovement
  (bind _mainstatsstructure (Variables|Default|GetMainStatsStructure))
  (bind _maxwalkspeed (Utilities|Struct|BreakSTRUCT_MainStats _mainstatsstructure))
  (if (Utilities|Enum|NotEqual(Enum) (.Type (Utilities|Struct|BreakSTRUCT_MainStats (Variables|Default|GetMainStatsStructure))) "NewEnumerator5")
    (bind _ascharacter (Utilities|Casting|CastToCharacter (Components|GetOwner)))
    (Variables|/Script/Engine.CharacterMovementComponent|SetMaxWalkSpeed (Variables|/Script/Engine.Character|GetCharacterMovement _ascharacter) _maxwalkspeed)
    (Variables|/Script/Engine.CharacterMovementComponent|SetMaxWalkSpeedCrouched (Variables|/Script/Engine.Character|GetCharacterMovement _ascharacter) (/ _maxwalkspeed 2.0))))

(fn ConfigureHealthandEPandFury
  (bind _savegameobject (Utilities|CheckSaveGame)
    (:Is%20Valid
      (Variables|Default|SetCurrentHP (Variables|/Game/Blueprints/Objects/BP_SaveGame.BP_SaveGame_C|GetSavedPlayerHP _savegameobject))
      (Variables|Default|SetCurrentEP (Variables|/Game/Blueprints/Objects/BP_SaveGame.BP_SaveGame_C|GetSavedPlayerEP _savegameobject))
      (Variables|Default|SetCurrentFury (Variables|/Game/Blueprints/Objects/BP_SaveGame.BP_SaveGame_C|GetSavedPlayerFury _savegameobject))
      (Variables|Default|SetCurrentStunLevel (Variables|/Game/Blueprints/Objects/BP_SaveGame.BP_SaveGame_C|GetSavedPlayerStunLevel _savegameobject))
      (Variables|Default|SetCurrentSummonLevel (Variables|/Game/Blueprints/Objects/BP_SaveGame.BP_SaveGame_C|GetSavedPlayerSummonLevel _savegameobject))
      (Variables|Default|SetTotalFuryPoints (Variables|/Game/Blueprints/Objects/BP_SaveGame.BP_SaveGame_C|GetSavedPlayerTotalFury _savegameobject))
      (Variables|Default|SetCurrentFuryLevelPoints (Variables|/Game/Blueprints/Objects/BP_SaveGame.BP_SaveGame_C|GetSavedPlayerLevelPoints _savegameobject))
      (Default|CallOnTotalFuryIncrease (Variables|Default|GetTotalFuryPoints))
      (Default|CallOnStatsUpdated (Variables|Default|GetCurrentHP) (Variables|Default|GetCurrentEP) (Variables|Default|GetIsDead) false (Variables|Default|GetCurrentFury)))
    (:False
      (CallFunction|HealUp true)
      (CallFunction|ShieldUP false)
      (CallFunction|FuryUporDown false 0 true))))

(fn UpdateBehavior
  (params (InCurrentBehavior :type ENUM_Behavior%20Enum :default "NewEnumerator0"))
  (Variables|Default|SetCurrentBehavior InCurrentBehavior))

(fn UpdateFraction
  (params (InCurrentFraction :type ENUM_Fractions%20Enum :default "NewEnumerator0"))
  (Variables|Default|SetCurrentFraction InCurrentFraction))

(fn ConfigureBehaviorandFraction
  (CallFunction|UpdateBehavior (.Behavior (Utilities|Struct|BreakSTRUCT_MainStats (Variables|Default|GetMainStatsStructure))))
  (CallFunction|UpdateFraction (.Fractions (Utilities|Struct|BreakSTRUCT_MainStats (Variables|Default|GetMainStatsStructure)))))

(fn FuryUporDown
  (params (InToMaximum :type Boolean) (InFuryPoints :type Integer) (IsItIncrease :type Boolean))
  (if IsItIncrease
    (Variables|Default|SetTotalFuryPoints (+ InFuryPoints (Variables|Default|GetTotalFuryPoints)))
    (if InToMaximum
      (Variables|Default|SetCurrentFury (Utilities|Struct|BreakSTRUCT_MainStats (Variables|Default|GetMainStatsStructure)))
      (else
        (Variables|Default|SetCurrentFury (Math|Integer|Min(Integer) (+ (Variables|Default|GetCurrentFury) InFuryPoints) (Utilities|Struct|BreakSTRUCT_MainStats (Variables|Default|GetMainStatsStructure))))))
    (Default|CallOnTotalFuryIncrease (Variables|Default|GetTotalFuryPoints))
    (EventDispatchers|BindEventtoOnTotalFuryIncrease (EventDispatchers|CreateEvent :!event LevelingSystemFunction))
    (Default|CallOnStatsUpdated (Variables|Default|GetCurrentHP) (Variables|Default|GetCurrentEP) (Variables|Default|GetIsDead) false (Variables|Default|GetCurrentFury))
    (elif (<= InFuryPoints (Variables|Default|GetCurrentFury))
      (bind _output_get (Variables|Default|SetCurrentFury (- (Variables|Default|GetCurrentFury) InFuryPoints)))
      (if (>= _output_get 0)
        _
        (else
          (Variables|Default|SetCurrentFury 0)))
      (Default|CallOnStatsUpdated (Variables|Default|GetCurrentHP) (Variables|Default|GetCurrentEP) (Variables|Default|GetIsDead) false (Variables|Default|GetCurrentFury))
      (return true)
      (else
        (return false)))))

(fn CheckFury
  (return (== (Variables|Default|GetCurrentFury) (.MaxFury (Utilities|Struct|BreakSTRUCT_MainStats (Variables|Default|GetMainStatsStructure))))))

(fn LevelingSystemFunction
  (params (TotalFuryPoints :type Integer))
  (Utilities|FlowControl|Sequence
    (:then_0
      (bind _isnewlevel (CallFunction|CheckIsNewLevel TotalFuryPoints (Variables|Default|GetCurrentFuryLevel)))
      (if _isnewlevel
        (bind _output_get (Variables|Default|SetCurrentFuryLevelPoints (+ (Variables|Default|GetCurrentFuryLevelPoints) 1)))
        (Default|CallOnCurrentFuryLevelPointsUpdated _output_get)))
    (:then_1
      (bind _foundwidgets (Widget|GetAllWidgetsOfClass "/Game/Blueprints/HUD/Widgets/W_SkillTree.W_SkillTree_C" false))
      (EventDispatchers|BindEventtoOnFuryLevelPointsDecreased _foundwidgets (EventDispatchers|CreateEvent :!event GetLevelPointsAfterUsage)))))

(fn CheckIsNewLevel
  (params (InTotalFury :type Integer) (InCurrentLevelName :type Name))
  (Variables|Default|SetLevelingStarted true)
  (if (== (Variables|Default|GetCurrentFuryLevel) "0LVL")
    (Variables|Default|SetNumberForNextLevel (+ 0 1)))
  (bind _output_get (Variables|Default|SetNextLevelName (Utilities|String|StringToName (Utilities|String|ToString(Text) (Utilities|Text|FormatText "{Number}LVL" (Variables|Default|GetNumberForNextLevel))))))
  (bind _returnvalue (Utilities|GetDataTableRow "/Game/Data/DT_Leveling.DT_Leveling" _output_get)
    (:then
      (bind _output_get_2 (LocalVariables|SetL_LevelingData _returnvalue))
      (bind _output_get_3 (Variables|Default|SetTotalFuryToGet (.TotalFuryToGet (Utilities|Struct|BreakSTRUCT_Leveling _output_get_2))))
      (if (>= InTotalFury _output_get_3)
        (Variables|Default|SetNumberForLevel (+ 1 (Variables|Default|GetNumberForLevel)))
        (Variables|Default|SetCurrentFuryLevel (Utilities|String|StringToName (Utilities|String|ToString(Text) (Utilities|Text|FormatText "{Number}LVL" (Variables|Default|GetNumberForLevel)))))
        (Variables|Default|SetNumberForNextLevel (+ 1 (Variables|Default|GetNumberForNextLevel)))
        (return true (Variables|Default|GetCurrentFuryLevel))
        (else
          (return false (Variables|Default|GetCurrentFuryLevel)))))))

(fn ConfigureNextLevelInfo
  (if (== (Variables|Default|GetCurrentName) "Player")
    (if (not (Variables|Default|GetLevelingStarted))
      (Variables|Default|SetTotalFuryToGet 100)
      (return)
      (else
        (return)))
    (else
      (return))))

(fn GetLevelPointsAfterUsage
  (params (CurrentLevelPoints :type Integer))
  (Variables|Default|SetCurrentFuryLevelPoints CurrentLevelPoints))