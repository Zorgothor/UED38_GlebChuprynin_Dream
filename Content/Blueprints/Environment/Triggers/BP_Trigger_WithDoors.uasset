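; Trigger Blueprint that toggles the locks on a set of linked doors when the player character overlaps it.
; After running the parent overlap logic, it validates the OverlappedActor variable and casts it to BP_PlayerCharacter.
; SwitchDoorsLock then calls SwitchLock on each door in DoorsToLockSwitch.
; With OnlyFirstActivation set, the AlreadyActive flag limits this to one activation; otherwise every qualifying overlap switches the locks again.
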(event EventBeginPlay
  (|CallParentFunction) ; Этот узел отключен и не будет вызываться.\nПеретащите контакты, чтобы построить функционал.
)

(event Collision|EventActorBeginOverlap
  (params (OtherActor :type Actor%20Object%20Reference))
  (|CallParentFunction OtherActor)
  (bind _overlappedactor (Variables|Default|GetOverlappedActor)
    (:then
      (Utilities|Casting|CastToBP_PlayerCharacter _overlappedactor)
      (CallFunction|SwitchDoorsLock))
    (:else)))

(event EventTick
  (params (DeltaSeconds :type Float%20%28single-precision%29))
  (|CallParentFunction DeltaSeconds) ; Этот узел отключен и не будет вызываться.\nПеретащите контакты, чтобы построить функционал.
)

(fn ConstructionScript
  (|CallParentFunction))

(fn SwitchDoorsLock
  (if (Variables|Default|GetOnlyFirstActivation)
    (if (not (Variables|Default|GetAlreadyActive))
      (Variables|Default|SetAlreadyActive true)
      (for _array_element (Variables|Default|GetDoorsToLockSwitch) :!label _label
        (Default|SwitchLock _array_element)))
    (else
      (goto _label))))