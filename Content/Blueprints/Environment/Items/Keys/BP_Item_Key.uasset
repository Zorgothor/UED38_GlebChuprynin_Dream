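; BP_Item_Key is a key item Blueprint that registers itself as a quest item when picked up into the backpack.
; It inherits its lifecycle, overlap and construction logic from a parent item class, forwarding those events unchanged.
; Its PutInToBackpack override calls the parent, adds its ItemName to the backpack's quest items, then calls AfterUse.
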(event EventBeginPlay
  (|CallParentFunction))

(event Collision|EventActorBeginOverlap
  (params (OtherActor :type Actor%20Object%20Reference))
  (|CallParentFunction OtherActor))

(event EventTick
  (params (DeltaSeconds :type Float%20%28single-precision%29))
  (|CallParentFunction DeltaSeconds))

(event Collision|EventActorEndOverlap
  (params (OtherActor :type Actor%20Object%20Reference))
  (|CallParentFunction OtherActor))

(fn ConstructionScript
  (|CallParentFunction))

(fn PutintoBackpack
  (params (InBackpack :type BP%20Back%20Pack%20Component%20Object%20Reference))
  (|CallParentFunction InBackpack)
  (Default|AddQuestItem InBackpack (Variables|Default|GetItemName))
  (CallFunction|AfterUse))