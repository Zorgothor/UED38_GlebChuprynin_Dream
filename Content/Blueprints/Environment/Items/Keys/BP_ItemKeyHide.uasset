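; BP_ItemKeyHide is a key item that stays hidden while any NPC belongs to a particular fraction.
; A looping three-second timer from BeginPlay gathers all BP_NPCCharacter actors and checks each stats component's CurrentFraction.
; The first match hides the mesh and text and clears the array to cut the loop short; otherwise both are shown.
; Only visibility changes, and the Tick timer-handle check does nothing.
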(event Custom|CustomEvent
  (bind _outactors (Actor|GetAllActorsOfClass "/Game/Blueprints/Character/NPC/BP_NPCCharacter.BP_NPCCharacter_C"))
  (bind _output_get (Variables|Default|SetNPCs _outactors))
  (if (Utilities|Array|IsNotEmpty (Variables|Default|GetNPCs))
    (for _array_element _output_get
      (if (not (Utilities|Enum|Equal(Enum) (Variables|/Game/Blueprints/Components/BP_MainStatsComponent.BP_MainStatsComponent_C|GetCurrentFraction (Variables|/Game/Blueprints/Character/BP_CharacterBase.BP_CharacterBase_C|GetBP_MainStatsComponent _array_element)) "NewEnumerator0"))
        (Rendering|SetVisibility (Variables|Default|GetItemMesh) true false)
        (else
          (Rendering|SetVisibility (Variables|Default|GetTextRender) false false)
          (Utilities|Array|Clear (Variables|Default|GetNPCs)))))
    (else
      (Rendering|SetVisibility (Variables|Default|GetTextRender) true false))))

(event EventBeginPlay
  (|CallParentFunction)
  (Utilities|Time|SetTimerbyEvent (delegate Custom|CustomEvent) 3.0 true))

(event Collision|EventActorBeginOverlap
  (params (OtherActor :type Actor%20Object%20Reference))
  (|CallParentFunction OtherActor) ; This node is disabled and will not be called.\nDrag off pins to build functionality.
)

(event EventTick
  (params (DeltaSeconds :type Float%20%28single-precision%29))
  (|CallParentFunction DeltaSeconds)
  (if (not (Utilities|Time|IsValidTimerHandle (Variables|Default|GetTimer)))
    _))

(fn ConstructionScript
  (|CallParentFunction))