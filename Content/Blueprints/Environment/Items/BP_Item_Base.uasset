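; Base pickup item that bobs and spins in the world and can be interacted with by a nearby character.
; Overlapping characters enable interaction and reveal a text prompt that turns toward the player camera.
; Tick drives an eased ping-pong float and constant yaw spin from a randomized initial rotation.
; Interact passes the character's backpack component to the empty PutInToBackpack hook; AfterUse plays a pickup sound and destroys the item.
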(event EventBeginPlay
  (Rendering|SetVisibility (Variables|Default|GetTextRender) false true)
  (Variables|Default|SetInitialLocation (Transformation|GetWorldLocation (Variables|Default|GetSphereCollision)))
  (Transformation|AddRelativeRotation (Variables|Default|GetSphereCollision) (Math|Rotator|MakeRotator 0.0 0.0 (Math|Random|RandomFloatinRange -9e+01 9e+01)) false false))

(event Collision|EventActorBeginOverlap
  (params (OtherActor :type Actor%20Object%20Reference))
  (bind _ascharacter (Utilities|Casting|CastToCharacter OtherActor))
  (Variables|Default|SetCharacterInBox _ascharacter)
  (Rendering|SetVisibility (Variables|Default|GetTextRender) true true)
  (Variables|Default|SetIsReadyToInteract true)
  (Variables|Default|SetLookAt true))

(event EventTick
  (params (DeltaSeconds :type Float%20%28single-precision%29))
  (Variables|Default|SetDeltaSeconds DeltaSeconds)
  (CallFunction|LookatPlayerCamera)
  (CallFunction|FloatandRotate))

(event Collision|EventActorEndOverlap
  (params (OtherActor :type Actor%20Object%20Reference))
  (Utilities|Casting|CastToCharacter OtherActor)
  (Variables|Default|SetCharacterInBox 0)
  (Rendering|SetVisibility (Variables|Default|GetTextRender) false true)
  (Variables|Default|SetIsReadyToInteract false)
  (Variables|Default|SetLookAt false))

(fn ConstructionScript)

(fn LookatPlayerCamera
  (if (Variables|Default|GetLookAt)
    (bind _characterinbox (Variables|Default|GetCharacterInBox)
      (:then
        (bind _asbp_player_character (Utilities|Casting|CastToBP_PlayerCharacter _characterinbox))
        (LocalVariables|SetCameraLocation%20 (Transformation|GetWorldLocation (Variables|/Game/Blueprints/Character/Player/BP_PlayerCharacter.BP_PlayerCharacter_C|GetCamera _asbp_player_character)))
        (Transformation|SetWorldRotation (Variables|Default|GetTextRender) (Math|Rotator|FindLookatRotation (Transformation|GetWorldLocation (Variables|Default|GetTextRender)) (LocalVariables|GetCameraLocation%20)) false false))
      (:else))))

(fn PutintoBackpack
  (params (InBackpack :type BP%20Back%20Pack%20Component%20Object%20Reference)))

(fn AfterUse
  (Audio|PlaySound2D "/Game/Retro_8Bit_Sounds/Collectables/Cues/retro_collect_pickup_coin_15_Cue.retro_collect_pickup_coin_15_Cue" 1.0 1.0 0.0 0 self)
  (Actor|DestroyActor))

(fn FloatandRotate
  (bind _initiallocation (Variables|Default|GetInitialLocation))
  (Utilities|FlowControl|Sequence
    (:then_0
      (if (not (Math|Float|NearlyEqual(Float) (Variables|Default|GetAlphaCurrent) (Math|Float|SelectFloat (Variables|Default|GetAlphaTarget) (Variables|Default|GetAlphaStart) (Variables|Default|GetAlphaForward)) 0.05))
        (Variables|Default|SetAlphaCurrent (Math|Float|SelectFloat (+ (Variables|Default|GetAlphaCurrent) (Variables|Default|GetDeltaSeconds)) (- (Variables|Default|GetAlphaCurrent) (Variables|Default|GetDeltaSeconds)) (Variables|Default|GetAlphaForward)))
        (else
          (Variables|Default|SetAlphaForward (not (Variables|Default|GetAlphaForward)))))
      (Transformation|SetWorldLocation (Variables|Default|GetSphereCollision) (Math|Interpolation|Ease "EaseInOut" (Variables|Default|GetAlphaCurrent) (Variables|Default|GetInitialLocation) (Math|Vector|MakeVector (.x _initiallocation) (.y _initiallocation) (+ (.z _initiallocation) (Variables|Default|GetLocationOffsetZ))) 2.0) false false))
    (:then_1
      (Transformation|AddRelativeRotation (Variables|Default|GetSphereCollision) (Math|Rotator|MakeRotator 0.0 0.0 (Variables|Default|GetRotationSpeed)) false false))))

(fn Interact
  (if (Variables|Default|GetIsReadyToInteract)
    (bind _characterinbox (Variables|Default|GetCharacterInBox)
      (:then
        (Utilities|IsValid (Actor|GetComponentbyClass _characterinbox "/Game/Blueprints/Components/BP_BackPackComponent.BP_BackPackComponent_C")
          (:Is%20Valid
            (CallFunction|PutintoBackpack (Actor|GetComponentbyClass _characterinbox "/Game/Blueprints/Components/BP_BackPackComponent.BP_BackPackComponent_C"))
            (return true))
          (:Is%20Not%20Valid
            (return true))))
      (:else
        (return true)))
    (else
      (return true))))