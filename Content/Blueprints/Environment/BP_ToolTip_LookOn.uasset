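; BP_ToolTip_LookOn is an environment tooltip actor whose text turns to face the player's camera while a character is in range.
; Overlap begin calls the parent, then sets a LookAt flag if CharacterInBox is valid; any overlap end clears it.
; Each tick, while flagged, it casts CharacterInBox to BP_PlayerCharacter and rotates ToolTipText toward that camera using FindLookAtRotation.
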(event EventBeginPlay
  (|CallParentFunction) ; Этот узел отключен и не будет вызываться.\nПеретащите контакты, чтобы построить функционал.
)

(event Collision|EventActorBeginOverlap
  (params (OtherActor :type Actor%20Object%20Reference))
  (|CallParentFunction OtherActor)
  (Variables|Default|GetCharacterInBox
    (:then
      (Variables|Default|SetLookAt true))
    (:else)))

(event EventTick
  (params (DeltaSeconds :type Float%20%28single-precision%29))
  (|CallParentFunction DeltaSeconds)
  (CallFunction|LookatPlayerCamera))

(event Collision|EventActorEndOverlap
  (params (OtherActor :type Actor%20Object%20Reference))
  (|CallParentFunction OtherActor)
  (Variables|Default|SetLookAt false))

(fn ConstructionScript
  (|CallParentFunction))

(fn LookatPlayerCamera
  (if (Variables|Default|GetLookAt)
    (bind _characterinbox (Variables|Default|GetCharacterInBox)
      (:then
        (bind _asbp_player_character (Utilities|Casting|CastToBP_PlayerCharacter _characterinbox))
        (Variables|Default|SetCameraLocation%20 (Transformation|GetWorldLocation (Variables|/Game/Blueprints/Character/Player/BP_PlayerCharacter.BP_PlayerCharacter_C|GetCamera _asbp_player_character)))
        (Transformation|SetWorldRotation (Variables|Default|GetToolTipText) (Math|Rotator|FindLookatRotation (Transformation|GetWorldLocation (Variables|Default|GetToolTipText)) (Variables|Default|GetCameraLocation%20)) false false))
      (:else))))