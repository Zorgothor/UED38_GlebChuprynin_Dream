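; Base Blueprint for weapon pickup items, defining what happens when one is put into a backpack.
; The PutInToBackpack override calls the parent, then uses ItemName to check the backpack's available weapons.
; An owned weapon gets an ammo increase equal to its max rounds, while a new one is added to the backpack.
; Either branch finishes with AfterUse, and an unset ItemName skips both steps.
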(event EventBeginPlay
  (|CallParentFunction) ; This node is disabled and will not be called.\nDrag off pins to build functionality.
)

(event Collision|EventActorBeginOverlap
  (params (OtherActor :type Actor%20Object%20Reference))
  (|CallParentFunction OtherActor) ; This node is disabled and will not be called.\nDrag off pins to build functionality.
)

(event EventTick
  (params (DeltaSeconds :type Float%20%28single-precision%29))
  (|CallParentFunction DeltaSeconds) ; This node is disabled and will not be called.\nDrag off pins to build functionality.
)

(fn ConstructionScript
  (|CallParentFunction))

(fn PutintoBackpack
  (params (InBackpack :type BP%20Back%20Pack%20Component%20Object%20Reference))
  (bind _output_get (LocalVariables|SetL_BackPack InBackpack))
  (|CallParentFunction _output_get)
  (if (!= (Variables|Default|GetItemName) "")
    (Utilities|FlowControl|Sequence
      (:then_0
        (if (.ReturnValue (Utilities|Map|Find (Variables|/Game/Blueprints/Components/BP_BackPackComponent.BP_BackPackComponent_C|GetAvailableWeapons (LocalVariables|GetL_BackPack)) (Variables|Default|GetItemName)))
          (Default|UpdateAmmobyName (LocalVariables|GetL_BackPack) (.RooundsMax (Default|GetMaxRoundsforWeapons (LocalVariables|GetL_BackPack) (Variables|Default|GetItemName))) true (Variables|Default|GetItemName))
          (else
            (Default|AddWeaponItem (LocalVariables|GetL_BackPack) (Variables|Default|GetItemName)))))
      (:then_1
        (CallFunction|AfterUse)))))