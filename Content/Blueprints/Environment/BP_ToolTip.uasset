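; BP_ToolTip is a placeable world tooltip that shows text and plays a sound while a Character stands inside its trigger box.
; Overlap events store or clear the character reference and toggle the text's visibility.
; The construction script applies the message and text position, then sizes the box and raises it by its Z extent so its bottom sits at the actor's origin.
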(event EventBeginPlay)

(event Collision|EventActorBeginOverlap
  (params (OtherActor :type Actor%20Object%20Reference))
  (bind _ascharacter (Utilities|Casting|CastToCharacter OtherActor))
  (Variables|Default|SetCharacterInBox _ascharacter)
  (Development|SetHiddeninGame (Variables|Default|GetToolTipText) false true)
  (Audio|Components|Audio|Play (Variables|Default|GetTipSound) 0.0))

(event EventTick
  (params (DeltaSeconds :type Float%20%28single-precision%29)))

(event Collision|EventActorEndOverlap
  (params (OtherActor :type Actor%20Object%20Reference))
  (Utilities|Casting|CastToCharacter OtherActor)
  (Variables|Default|SetCharacterInBox 0)
  (Development|SetHiddeninGame (Variables|Default|GetToolTipText) true true))

(fn ConstructionScript
  (CallFunction|CollisionfromFloor)
  (Transformation|SetRelativeLocation (Variables|Default|GetToolTipText) (Variables|Default|GetToolTipTextLocation) false false)
  (Rendering|Components|TextRender|SetText (Variables|Default|GetToolTipText) (Variables|Default|GetToolTipTextMassage)))

(fn CollisionfromFloor
  (Components|Box|SetBoxExtent (Variables|Default|GetBoxCollision) (Variables|Default|GetBoxExtent) true)
  (Transformation|SetRelativeLocation (Variables|Default|GetBoxCollision) (Math|Vector|MakeVector 0.0 0.0 (.Z (Math|Vector|BreakVector (Variables|Default|GetBoxExtent)))) false false))