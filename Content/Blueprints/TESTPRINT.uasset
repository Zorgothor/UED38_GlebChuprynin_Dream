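; Test actor Blueprint that prints a boolean to the screen on BeginPlay.
; BeginPlay calls a custom event twice, first with defaults and then with true; the print's color follows the value, green or red.
; An unconnected, never-run traffic-light loop would show an enum on a TextRender and cycle Stop, Ready and Go after a delay.
; Tick, overlap, the construction script and NewFunction are empty.
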(event Custom|CustomEvent
  (params (NewParam :type Boolean) (NewParam2 :type Name) (NewParam3 :type Integer) (NewParam4 :type Float%20%28double-precision%29))
  (Development|PrintString (Utilities|String|ToString(Boolean) NewParam) true true (Math|Color|SelectColor "(R=0.638653,G=1.000000,B=0.000000,A=1.000000)" "(R=1.000000,G=0.000000,B=0.000000,A=1.000000)" NewParam) 7.0))

(event EventBeginPlay
  (CallFunction|CustomEvent false "None" 0 0.0)
  (CallFunction|CustomEvent true "None" 0 0.0))

(event Collision|EventActorBeginOverlap
  (params (OtherActor :type Actor%20Object%20Reference)))

(event EventTick
  (params (DeltaSeconds :type Float%20%28single-precision%29)))

(fn ConstructionScript)

(fn NewFunction)