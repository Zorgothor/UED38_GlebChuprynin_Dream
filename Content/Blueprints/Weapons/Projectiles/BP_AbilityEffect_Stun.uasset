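; Stun ability blast actor that damages and stuns NPCs around its location when spawned.
; A recursive sphere trace on BeginPlay finds targets one by one, growing its ignore list each pass.
; Each hit gets a distance-scaled or radial impulse, damage from the player's stun-level data table row, and NPC AI controllers receive stun state and duration.
; A timer handles cleanup, with destruction gated on the explosion sound having finished.
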(event EventBeginPlay
  (Utilities|FlowControl|Sequence
    (:then_0
      (CallFunction|SphereTraceCheck))
    (:then_1
      (bind _returnvalue (Utilities|Time|SetTimerbyEvent (EventDispatchers|CreateEvent :!event ReadytoDestroy) 1.0))
      (Variables|Default|SetDestroyHandler _returnvalue))))

(event Collision|EventActorBeginOverlap
  (params (OtherActor :type Actor%20Object%20Reference)))

(event EventTick
  (params (DeltaSeconds :type Float%20%28single-precision%29)))

(fn ConstructionScript)

(fn SphereTraceCheck
  (bind _self self)
  (bind _returnvalue (Transformation|GetActorLocation _self))
  (bind (_outhit _returnvalue_2) (Collision|SphereTraceForObjects _returnvalue (+ _returnvalue "0.000000,0.000000,1.000000") (Variables|/Script/Engine.SphereComponent|GetSphereRadius (Variables|Default|GetSphereCollision)) (Utilities|Array|MakeArray "ObjectTypeQuery2" "ObjectTypeQuery3" "ObjectTypeQuery4") false (Variables|Default|GetInExplosionActor) "None"))
  (if _returnvalue_2
    (bind _output_get (Variables|Default|SetHitActor (.HitActor (Collision|BreakHitResult _outhit))))
    (Utilities|Array|AddUnique (Variables|Default|GetInExplosionActor) _output_get)
    (Variables|Default|SetHitComponent (.HitComponent (Collision|BreakHitResult _outhit)))
    (Utilities|FlowControl|Sequence
      (:then_0
        (CallFunction|AddImpulse))
      (:then_1
        (CallFunction|MakeDamage))
      (:then_2
        (CallFunction|SphereTraceCheck)))))

(fn ReadytoDestroy
  (if (not (Audio|Components|Audio|IsPlaying (Variables|Default|GetExplosionSFX)))
    (if (Utilities|Time|IsValidTimerHandle (Variables|Default|GetDestroyHandler))
      (Utilities|Time|ClearandInvalidateTimerbyHandle (Variables|Default|GetDestroyHandler))
      (Actor|DestroyActor))))

(fn AddImpulse
  (bind _returnvalue (Transformation|GetActorLocation))
  (bind _hitactor (Variables|Default|GetHitActor))
  (bind _returnvalue_2 (Transformation|GetActorLocation _hitactor))
  (bind _returnvalue_3 (- _returnvalue_2 _returnvalue))
  (bind _hitcomponent (Variables|Default|GetHitComponent)
    (:then
      (if (Physics|IsSimulatingPhysics _hitcomponent "None")
        (Physics|AddImpulseatLocation (Variables|Default|GetHitComponent) (* _returnvalue_3 (Math|Float|Absolute(Float) (* (Math|Float|MapRangeClamped (Math|Vector|VectorLength _returnvalue_3) 0.0 (Variables|/Script/Engine.SphereComponent|GetSphereRadius (Variables|Default|GetSphereCollision)) 1.0 0.5) (Variables|Default|GetImpulsMult)))) (Transformation|GetActorLocation) "None")
        (else
          (Class|RadialForceComponent|FireImpulse (Variables|Default|GetRadialForce)))))
    (:else)))

(fn MakeDamage
  (bind _asbp_player_character (Utilities|Casting|CastToBP_PlayerCharacter (Components|GetOwner (Components|GetOwner))))
  (bind _returnvalue (Utilities|GetDataTableRow "/Game/Data/DT_AbilityInfo.DT_AbilityInfo" (Variables|/Game/Blueprints/Components/BP_MainStatsComponent.BP_MainStatsComponent_C|GetCurrentStunLevel (Variables|/Game/Blueprints/Character/BP_CharacterBase.BP_CharacterBase_C|GetBP_MainStatsComponent _asbp_player_character)))
    (:then
      (Variables|Default|SetCurrentStunStats _returnvalue)
      (Variables|Default|GetHitActor
        (:then
          (Variables|Default|SetStunTime (.StunTime (Utilities|Struct|BreakAbilityStats (Variables|Default|GetCurrentStunStats))))
          (Game|Damage|ApplyDamage (Variables|Default|GetHitActor) (Math|Conversions|ToFloat(Integer) (.DamageFromStun (Utilities|Struct|BreakAbilityStats (Variables|Default|GetCurrentStunStats)))) 0 (Components|GetOwner) "/Game/Blueprints/Objects/BP_DamageObject.BP_DamageObject_C")
          (bind _asbp_npccharacter (Utilities|Casting|CastToBP_NPCCharacter (Variables|Default|GetHitActor)))
          (bind _asbp_aicontroller (Utilities|Casting|CastToBP_AIController (Pawn|GetController _asbp_npccharacter)))
          (Variables|/Game/Blueprints/Controller/BP_AIController.BP_AIController_C|SetStunDuration _asbp_aicontroller (Variables|Default|GetStunTime))
          (Variables|/Game/Blueprints/Controller/BP_AIController.BP_AIController_C|SetIsItNewStun _asbp_aicontroller true)
          (Variables|/Game/Blueprints/Controller/BP_AIController.BP_AIController_C|SetAIState%20 _asbp_aicontroller "NewEnumerator6"))
        (:else)))))