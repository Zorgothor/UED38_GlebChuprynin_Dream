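; Stun ability projectile that spawns a BP_AbilityEffect_Stun actor at its transform when it hits, then destroys itself.
; When owned by BP_PlayerCharacter, BeginPlay boosts velocity once along its heading using an exponentiated Acceleration.
; It also starts a looping timer on AddSpeed, which is empty.
; Empty SpawnDecal and ApplyDamageByProjectile overrides skip the parent's decal and damage logic, and OnEndOfHit is empty too.
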(event Custom|AddSpeed)

(event EventBeginPlay
  (|CallParentFunction)
  (Utilities|Casting|CastToBP_PlayerCharacter (Components|GetOwner))
  (Utilities|Time|SetTimerbyEvent (delegate Custom|AddSpeed) 0.1 true)
  (Variables|Default|SetAcceleration (Math|Float|Power (Variables|Default|GetAcceleration) 1.2))
  (Variables|/Script/Engine.MovementComponent|SetVelocity (Variables|Default|GetProjectileMovement) (+ (* (Math|Vector|Normalize (Variables|/Script/Engine.MovementComponent|GetVelocity (Variables|Default|GetProjectileMovement))) (Variables|Default|GetAcceleration)) (Variables|/Script/Engine.MovementComponent|GetVelocity (Variables|Default|GetProjectileMovement)))))

(event Collision|EventActorBeginOverlap
  (params (OtherActor :type Actor%20Object%20Reference))
  (|CallParentFunction OtherActor) ; This node is disabled and will not be called.\nDrag off pins to build functionality.
)

(event EventTick
  (params (DeltaSeconds :type Float%20%28single-precision%29))
  (|CallParentFunction DeltaSeconds) ; This node is disabled and will not be called.\nDrag off pins to build functionality.
)

(event Collision|EventHit
  (params (MyComp :type Primitive%20Component%20Object%20Reference) (Other :type Actor%20Object%20Reference) (OtherComp :type Primitive%20Component%20Object%20Reference) (bSelfMoved :type Boolean) (HitLocation :type Vector :default "0, 0, 0") (HitNormal :type Vector :default "0, 0, 0") (NormalImpulse :type Vector :default "0, 0, 0") (Hit :type Hit%20Result%20Structure%20%28by%20ref%29))
  (|CallParentFunction MyComp Other OtherComp bSelfMoved HitLocation HitNormal NormalImpulse Hit)
  (Game|SpawnActorfromClass "/Game/Blueprints/Weapons/Projectiles/BP_AbilityEffect_Stun.BP_AbilityEffect_Stun_C" (Transformation|GetActorTransform) "AlwaysSpawn" "MultiplyWithRoot" self 0)
  (Actor|DestroyActor))

(fn ConstructionScript
  (|CallParentFunction))

(fn SpawnDecal)

(fn OnEndOfHit)

(fn ApplyDamagebyProjectile)