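; Base weapon projectile that, on hit, applies physics impulse and damage, spawns an attached impact effect, then destroys itself.
; Impulse uses velocity on simulating components, otherwise fires a radial force.
; Damage comes from the owning BP_BaseWeapon, triples on head hits, and feeds half into the shooting player's Fury for listed limb bones on characters.
; A recursive parent-bone limb check exists but is not called here.
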(event EventBeginPlay)

(event Collision|EventActorBeginOverlap
  (params (OtherActor :type Actor%20Object%20Reference)))

(event EventTick
  (params (DeltaSeconds :type Float%20%28single-precision%29)))

(event Collision|EventHit
  (params (MyComp :type Primitive%20Component%20Object%20Reference) (Other :type Actor%20Object%20Reference) (OtherComp :type Primitive%20Component%20Object%20Reference) (bSelfMoved :type Boolean) (HitLocation :type Vector :default "0, 0, 0") (HitNormal :type Vector :default "0, 0, 0") (NormalImpulse :type Vector :default "0, 0, 0") (Hit :type Hit%20Result%20Structure%20%28by%20ref%29))
  (Variables|Default|SetHitLocation HitLocation)
  (Variables|Default|SetHitNormal HitNormal)
  (Variables|Default|SetOtherComp OtherComp)
  (Variables|Default|SetOther Other)
  (Development|PrintString (Utilities|GetDisplayName Other))
  (Variables|Default|SetHitResult Hit)
  (Utilities|FlowControl|Sequence
    (:then_0
      (CallFunction|AddPhysImpuls))
    (:then_1
      (CallFunction|ApplyDamagebyProjectile))
    (:then_2
      (CallFunction|SpawnDecal))
    (:then_3
      (CallFunction|OnEndOfHit))))

(fn ConstructionScript)

(fn OnEndOfHit
  (Actor|DestroyActor))

(fn ApplyDamagebyProjectile
  (bind _hitresult (Variables|Default|GetHitResult))
  (bind (_bblockinghit _binitialoverlap _time _distance _location _impactpoint _normal _impactnormal _physmat _hitactor _hitcomponent _hitbonename) (Collision|BreakHitResult _hitresult))
  (Utilities|FlowControl|Sequence
    (:then_0
      (bind _asbp_base_weapon (Utilities|Casting|CastToBP_BaseWeapon (Components|GetOwner)))
      (LocalVariables|SetL_CurrentDamage (Variables|/Game/Blueprints/Weapons/BP_BaseWeapon.BP_BaseWeapon_C|GetDamageCurrent _asbp_base_weapon)))
    (:then_1
      (Variables|Default|SetHitActor _hitactor)
      (Variables|Default|SetHitBone _hitbonename)
      (if (== _hitbonename "head")
        (LocalVariables|SetL_CurrentDamage (* (LocalVariables|GetL_CurrentDamage) 3))))
    (:then_2
      (bind _asbp_character_base (Utilities|Casting|CastToBP_CharacterBase (Variables|Default|GetHitActor)))
      (if (Utilities|Struct|BreakSTRUCT_MainStats (Variables|/Game/Blueprints/Components/BP_MainStatsComponent.BP_MainStatsComponent_C|GetMainStatsStructure (Variables|/Game/Blueprints/Character/BP_CharacterBase.BP_CharacterBase_C|GetBP_MainStatsComponent _asbp_character_base)))
        _
        (else
          _))
      (if (Utilities|Array|ContainsItem (Variables|Default|GetLimbsArray) (Variables|Default|GetHitBone))
        (bind _asbp_player_character (Utilities|Casting|CastToBP_PlayerCharacter (Components|GetOwner (Components|GetOwner))))
        (Default|FuryUporDown (Actor|GetComponentbyClass _asbp_player_character "/Game/Blueprints/Components/BP_MainStatsComponent.BP_MainStatsComponent_C") (== (/ (LocalVariables|GetL_CurrentDamage) 2) (.MaxFury (Utilities|Struct|BreakSTRUCT_MainStats (Variables|/Game/Blueprints/Components/BP_MainStatsComponent.BP_MainStatsComponent_C|GetMainStatsStructure (Actor|GetComponentbyClass _asbp_player_character "/Game/Blueprints/Components/BP_MainStatsComponent.BP_MainStatsComponent_C"))))) (/ (LocalVariables|GetL_CurrentDamage) 2) true)))
    (:then_3
      (Game|Damage|ApplyDamage (Variables|Default|GetOther) (Math|Conversions|ToFloat(Integer) (LocalVariables|GetL_CurrentDamage)) 0 (Components|GetOwner (Components|GetOwner)) "/Game/Blueprints/Objects/BP_DamageObject.BP_DamageObject_C"))))

(fn SpawnDecal
  (bind _hitnormal (Variables|Default|GetHitNormal))
  (bind _returnvalue (Math|Conversions|RotationFromXVector _hitnormal))
  (LocalVariables|SetL_Rotator (Math|Rotator|MakeRotator (Math|Random|RandomFloatinRange 0.0 3.6e+02) (.pitch _returnvalue) (.yaw _returnvalue)))
  (bind _returnvalue_2 (Game|SpawnActorfromClass "/Game/Blueprints/Weapons/Projectiles/BP_ShotImpactEffect.BP_ShotImpactEffect_C" (Math|Transform|MakeTransform (Variables|Default|GetHitLocation) (LocalVariables|GetL_Rotator) "1.000000,1.000000,1.000000") "Undefined" "MultiplyWithRoot" self 0))
  (LocalVariables|SetL_Impact _returnvalue_2)
  (Transformation|AttachComponentToComponent (LocalVariables|GetL_Impact) (Variables|Default|GetOtherComp) (.HitBoneName (Collision|BreakHitResult (Variables|Default|GetHitResult))) "KeepWorld" "KeepWorld" "KeepWorld" true))

(fn AddPhysImpuls
  (if (Variables|Impuls|GetIsMakingImpuls)
    (bind _othercomp (Variables|Default|GetOtherComp)
      (:then
        (if (Physics|IsSimulatingPhysics _othercomp "None")
          (Physics|AddImpulseatLocation (Variables|Default|GetOtherComp) (* (Transformation|GetVelocity) (Variables|Impuls|GetImpulsMult)) (Transformation|GetActorLocation) "None")
          (else
            (Class|RadialForceComponent|FireImpulse (Variables|Default|GetRadialForce)))))
      (:else))))

(fn CheckIsBoneLimb
  (params (InHitActor :type Actor%20Object%20Reference) (InBoneName :type Name))
  (bind _asbp_character_base (Utilities|Casting|CastToBP_CharacterBase InHitActor))
  (if (not (== (Class|SkinnedMeshComponent|GetParentBone (Actor|GetComponentbyClass _asbp_character_base "/Script/Engine.SkeletalMeshComponent") (Variables|Default|GetHitBone)) ""))
    (if (Math|Boolean|ORBoolean (== (Class|SkinnedMeshComponent|GetParentBone (Actor|GetComponentbyClass _asbp_character_base "/Script/Engine.SkeletalMeshComponent") (Variables|Default|GetHitBone)) "neck_01") (== (Class|SkinnedMeshComponent|GetParentBone (Actor|GetComponentbyClass _asbp_character_base "/Script/Engine.SkeletalMeshComponent") (Variables|Default|GetHitBone)) "UpperArm_R") (== (Class|SkinnedMeshComponent|GetParentBone (Actor|GetComponentbyClass _asbp_character_base "/Script/Engine.SkeletalMeshComponent") (Variables|Default|GetHitBone)) "UpperArm_L") (== (Class|SkinnedMeshComponent|GetParentBone (Actor|GetComponentbyClass _asbp_character_base "/Script/Engine.SkeletalMeshComponent") (Variables|Default|GetHitBone)) "Thigh_L") (== (Class|SkinnedMeshComponent|GetParentBone (Actor|GetComponentbyClass _asbp_character_base "/Script/Engine.SkeletalMeshComponent") (Variables|Default|GetHitBone)) "Thigh_R"))
      (Variables|Default|SetItIsLimb true)
      (return)
      (else
        (CallFunction|CheckIsBoneLimb (Variables|Default|GetHitActor) (Class|SkinnedMeshComponent|GetParentBone (Actor|GetComponentbyClass _asbp_character_base "/Script/Engine.SkeletalMeshComponent") (Variables|Default|GetHitBone)))))
    (else
      (return))))