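; Shotgun weapon that fires a horizontal fan of pellets per shot.
; SingleShot loops up to MaxBulletInShot, spawning BP_ProjectileShotgun actors at the Muzzle transform with the weapon as owner, then calls ShotFXs.
; Each pellet's yaw is offset by its index relative to half the count, scaled by a small random factor for uneven spread.
; The ShotAngle variable is unused, and the event graph holds only disabled stubs.
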(event EventBeginPlay
  (|CallParentFunction) ; This node is disabled and will not be called.\nDrag off pins to build functionality.
)

(event Collision|EventActorBeginOverlap
  (params (OtherActor :type Actor%20Object%20Reference))
  (|CallParentFunction OtherActor) ; This node is disabled and will not be called.\nDrag off pins to build functionality.
)

(event EventTick
  (params (DeltaSeconds :type Float%20%28single-precision%29))
  (|CallParentFunction DeltaSeconds) ; This node is disabled and will not be called.\nDrag off pins to build functionality.
)

(fn ConstructionScript
  (|CallParentFunction))

(fn SingleShot
  (bind _muzzle (Variables|Default|GetMuzzle))
  (bind _returnvalue (Transformation|GetWorldTransform _muzzle))
  (bind (_roll _pitch _yaw) (Math|Rotator|BreakRotator (.rotation _returnvalue)))
  (Utilities|FlowControl|Sequence
    (:then_0
      (for _index (range 0 (Variables|Default|GetMaxBulletInShot))
        (LocalVariables|SetL_Index _index)
        (Game|SpawnActorfromClass "/Game/Blueprints/Weapons/Projectiles/BP_ProjectileShotgun.BP_ProjectileShotgun_C" (Math|Transform|MakeTransform (.location _returnvalue) (Math|Rotator|MakeRotator _roll _pitch (+ _yaw (* (- (LocalVariables|GetL_Index) (/ (Variables|Default|GetMaxBulletInShot) 2)) (Math|Random|RandomFloatinRange 0.8 1.3)))) (.scale _returnvalue)) "AdjustIfPossibleButAlwaysSpawn" "MultiplyWithRoot" self 0)))
    (:then_1
      (CallFunction|ShotFXs))))