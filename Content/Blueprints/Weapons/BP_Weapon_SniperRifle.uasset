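; Sniper rifle weapon Blueprint that fires single hitscan shots from the muzzle.
; SingleShot line-traces along the muzzle's forward vector, stores the hit, then applies impulse, damage and an attached impact effect; ShotFXs runs even on a miss.
; Hits on the "head" bone deal triple damage.
; The optional impulse pushes simulating components directly or fires a RadialForce at non-simulating ones; trace debug drawing remains enabled.
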(event EventBeginPlay
  (|CallParentFunction) ; This node is disabled and will not be called.\nDrag off pins to build functionality.
)

(event Collision|EventActorBeginOverlap
  (params (OtherActor :type Actor%20Object%20Reference))
  (|CallParentFunction OtherActor) ; This node is disabled and will not be called.\nDrag off pins to build functionality.
)

(event EventTick
  (params (DeltaSeconds :type Float%20%28single-precision%29))
  (|CallParentFunction DeltaSeconds) ; This node is disabled and will not be called.\nDrag off pins to build functionality.
)

(fn ConstructionScript
  (|CallParentFunction))

(fn SingleShot
  (bind _muzzle (Variables|Default|GetMuzzle))
  (bind _returnvalue (Transformation|GetWorldLocation _muzzle))
  (Utilities|FlowControl|Sequence
    (:then_0
      (bind (_outhit _returnvalue_2) (Collision|LineTraceByChannel _returnvalue (+ (* (Math|Vector|GetForwardVector (Variables|Default|GetMuzzle)) 2.5e+04) _returnvalue) "TraceTypeQuery2" true (Utilities|Array|MakeArray self (Components|GetOwner)) "ForDuration" true "(R=1.000000,G=0.000000,B=0.000000,A=1.000000)" "(R=0.000000,G=1.000000,B=0.000000,A=1.000000)" 1e+01))
      (if _returnvalue_2
        (Rendering|Debug|DrawDebugSphere "0, 0, 0" 2e+01 12 "(R=0.000000,G=1.000000,B=0.063235,A=1.000000)" 1e+01 2.0)
        (Variables|Default|SetHitLocation (.Location (Collision|BreakHitResult _outhit)))
        (Variables|Default|SetHitNormal (.Normal (Collision|BreakHitResult _outhit)))
        (Variables|Default|SetHitActor (.HitActor (Collision|BreakHitResult _outhit)))
        (Variables|Default|SetHitComponent (.HitComponent (Collision|BreakHitResult _outhit)))
        (Variables|Default|SetHitBoneName (.HitBoneName (Collision|BreakHitResult _outhit)))
        (Utilities|FlowControl|Sequence
          (:then_0
            (CallFunction|AddPhysImpuls))
          (:then_1
            (Shooting|ApplyDamagebyHitScan))
          (:then_2
            (Shooting|SpawnDecal)))))
    (:then_1
      (CallFunction|ShotFXs))))

(fn ApplyDamagebyHitScan
  (Utilities|FlowControl|Sequence
    (:then_0
      (LocalVariables|SetL_CurrentDamage (Variables|Default|GetDamageCurrent)))
    (:then_1
      (if (== (Variables|Default|GetHitBoneName) "head")
        (LocalVariables|SetL_CurrentDamage (* (LocalVariables|GetL_CurrentDamage) 3))))
    (:then_2
      (Game|Damage|ApplyDamage (Variables|Default|GetHitActor) (Math|Conversions|ToFloat(Integer) (LocalVariables|GetL_CurrentDamage)) 0 (Components|GetOwner) "/Game/Blueprints/Objects/BP_DamageObject.BP_DamageObject_C"))))

(fn SpawnDecal
  (bind _hitnormal (Variables|Default|GetHitNormal))
  (bind _returnvalue (Math|Conversions|RotationFromXVector _hitnormal))
  (LocalVariables|SetL_Rotator (Math|Rotator|MakeRotator (Math|Random|RandomFloatinRange 0.0 3.6e+02) (.pitch _returnvalue) (.yaw _returnvalue)))
  (bind _returnvalue_2 (Game|SpawnActorfromClass "/Game/Blueprints/Weapons/Projectiles/BP_ShotImpactEffect.BP_ShotImpactEffect_C" (Math|Transform|MakeTransform (Variables|Default|GetHitLocation) (LocalVariables|GetL_Rotator) "1.000000,1.000000,1.000000") "Undefined" "MultiplyWithRoot" self 0))
  (LocalVariables|SetL_Impact _returnvalue_2)
  (Transformation|AttachComponentToComponent (LocalVariables|GetL_Impact) (Variables|Default|GetHitComponent) (Variables|Default|GetHitBoneName) "KeepWorld" "KeepWorld" "KeepWorld" true))

(fn AddPhysImpuls
  (if (Variables|Impuls|GetIsMakingImpuls)
    (bind _hitcomponent (Variables|Default|GetHitComponent)
      (:then
        (if (Physics|IsSimulatingPhysics _hitcomponent "None")
          (Physics|AddImpulseatLocation (Variables|Default|GetHitComponent) (* (* (Math|Vector|Normalize (- (Variables|Default|GetHitLocation) (Transformation|GetWorldLocation (Variables|Default|GetMuzzle)))) 2e+03) (Variables|Impuls|GetImpulsMult)) (Variables|Default|GetHitLocation) "None")
          (else
            (Transformation|SetWorldLocation (Variables|Default|GetRadialForce) (Variables|Default|GetHitLocation) false false)
            (Class|RadialForceComponent|FireImpulse (Variables|Default|GetRadialForce)))))
      (:else))))