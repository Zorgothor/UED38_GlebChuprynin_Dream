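; Base weapon actor that fires projectiles by weapon type, with ammo, reloading, muzzle FX and AI-audible noise.
; Stats come from DT_WeaponStats by name, with damage scaled by the owner's stats component and infinite ammo plus auto-reload forced for NPC owners.
; While active, Tick polls held fire input through a weapon state machine, using timers for shot and reload delays.
; Reload plays a montage and draws rounds from the owner's backpack unless ammo is infinite.
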(event EventBeginPlay)

(event Collision|EventActorBeginOverlap
  (params (OtherActor :type Actor%20Object%20Reference)))

(event EventTick
  (params (DeltaSeconds :type Float%20%28single-precision%29))
  (if (Variables|Configuration|GetIsWeaponActive)
    (Shooting|Shooting)))

(event EventShootProcess
  (params (InProcess :type Boolean))
  (Shooting|ShootInputRecieved InProcess))

(fn ConstructionScript)

(fn ConfigureWeaponStats
  (params (InWeaponName :type Name))
  (bind _returnvalue (Components|GetOwner))
  (Variables|Configuration|SetWeaponName InWeaponName)
  (if (!= (Variables|Configuration|GetWeaponName) "")
    (bind _returnvalue_2 (Utilities|GetDataTableRow "/Game/Data/DT_WeaponStats.DT_WeaponStats" (Variables|Configuration|GetWeaponName))
      (:then
        (Variables|Configuration|SetWeaponStats _returnvalue_2)
        (Utilities|FlowControl|Sequence
          (:then_0
            (Variables|Configuration|SetRoundsCurrent (.RooundsMax (Utilities|Struct|BreakSTRUCT_WeaponStats (Variables|Configuration|GetWeaponStats))))
            (Variables|Configuration|SetDamageCurrent (.Damage (Utilities|Struct|BreakSTRUCT_WeaponStats (Variables|Configuration|GetWeaponStats)))))
          (:then_1
            (CallFunction|UpdateCurrentInfinite (Utilities|Struct|BreakSTRUCT_WeaponStats (Variables|Configuration|GetWeaponStats)))
            (CallFunction|UpdateAutoReload (Utilities|Struct|BreakSTRUCT_WeaponStats (Variables|Configuration|GetWeaponStats))))
          (:then_2
            (Utilities|IsValid _returnvalue
              (:Is%20Valid
                (LocalVariables|SetL_Owner _returnvalue)
                (Utilities|FlowControl|Sequence
                  (:then_0
                    (Utilities|IsValid (Actor|GetComponentbyClass (LocalVariables|GetL_Owner) "/Game/Blueprints/Components/BP_MainStatsComponent.BP_MainStatsComponent_C")
                      (:Is%20Valid
                        (Variables|Configuration|SetDamageCurrent (Math|Float|Truncate (* (.DamageMult (Utilities|Struct|BreakSTRUCT_MainStats (Variables|/Game/Blueprints/Components/BP_MainStatsComponent.BP_MainStatsComponent_C|GetMainStatsStructure (Actor|GetComponentbyClass (LocalVariables|GetL_Owner) "/Game/Blueprints/Components/BP_MainStatsComponent.BP_MainStatsComponent_C")))) (Variables|Configuration|GetDamageCurrent)))))))
                  (:then_1
                    (Utilities|Casting|CastToBP_NPCCharacter (LocalVariables|GetL_Owner))
                    (CallFunction|UpdateCurrentInfinite true)
                    (CallFunction|UpdateAutoReload true)))))))))))

(fn Shooting
  (if (Variables|Configuration|GetInProcess)
    (if (Utilities|Enum|Equal(Enum) (Variables|Configuration|GetWeaponState) "NewEnumerator0")
      (Shooting|SingleShot)
      (bind _allowshooting (Reload|RoundsCount))
      (if _allowshooting
        (Utilities|Time|SetTimerbyEvent (EventDispatchers|CreateEvent :!event AfterShotDelayEnds) (.ShotTime (Utilities|Struct|BreakSTRUCT_WeaponStats (Variables|Configuration|GetWeaponStats))))
        (Variables|Configuration|SetWeaponState "NewEnumerator1")
        (Default|CallOnWeaponStatusChanged)
        (else
          (Variables|Configuration|SetWeaponState "NewEnumerator2")
          (if (Variables|Default|GetCurrentAutoReload)
            (Reload|Reload)
            (else
              (Default|CallOnWeaponStatusChanged)))))
      (else
        (switch Utilities|FlowControl|Switch|SwitchonENUM_WeaponState (Variables|Configuration|GetWeaponState)
          (:NewEnumerator2
            _)
          (:NewEnumerator4
            _))
        (if (not (Audio|Components|Audio|IsPlaying (Variables|Default|GetMissClick)))
          (Audio|Components|Audio|Play (Variables|Default|GetMissClick) 0.0))))))

(fn ShootInputRecieved
  (params (InProcess :type Boolean))
  (Variables|Configuration|SetInProcess InProcess))

(fn ActivateWeapon
  (params (Activation :type Boolean))
  (Variables|Configuration|SetIsWeaponActive Activation)
  (Utilities|FlowControl|Sequence
    (:then_0
      (bind _output_get (LocalVariables|SetL_SkelMesh (Actor|GetComponentsByClass "/Script/Engine.SkeletalMeshComponent")))
      (if (Utilities|Array|IsValidIndex _output_get)
        (for _array_element (LocalVariables|GetL_SkelMesh)
          (Rendering|SetVisibility _array_element (Variables|Configuration|GetIsWeaponActive) true))))
    (:then_1
      (bind _output_get_2 (LocalVariables|SetL_StatMesh (Actor|GetComponentsByClass "/Script/Engine.StaticMeshComponent")))
      (if (Utilities|Array|IsValidIndex _output_get_2)
        (for _array_element_2 (LocalVariables|GetL_StatMesh)
          (Rendering|SetVisibility _array_element_2 (Variables|Configuration|GetIsWeaponActive) true))))))

(fn SingleShot
  (Class|AISenseHearing|ReportNoiseEvent (Transformation|GetWorldLocation (Variables|Default|GetMuzzle)) 1.0 self 0.0 "None")
  (bind _returnvalue (Game|SpawnActorfromClass (Utilities|Select :Index (.WeaponType (Utilities|Struct|BreakSTRUCT_WeaponStats (Variables|Configuration|GetWeaponStats))) :NewEnumerator0 "/Game/Blueprints/Weapons/Projectiles/BP_ProjectilePistol.BP_ProjectilePistol_C" :NewEnumerator1 "/Game/Blueprints/Weapons/Projectiles/BP_ProjectileRifle.BP_ProjectileRifle_C" :NewEnumerator2 0 :NewEnumerator3 "/Game/Blueprints/Weapons/Projectiles/BP_ProjectileRocketLauncher.BP_ProjectileRocketLauncher_C" :NewEnumerator4 0) (Transformation|GetWorldTransform (Variables|Default|GetMuzzle)) "Undefined" "MultiplyWithRoot" self 0))
  (Utilities|Casting|CastToBP_ProjectileBase _returnvalue)
  (Shooting|ShotFXs))

(fn RoundsCount
  (bind _result (Math|Integer|DecrementInt (Variables|Configuration|GetRoundsCurrent))
    (:%20%20
      (return (> _result 0)))))

(fn AfterShotDelayEnds
  (Variables|Configuration|SetWeaponState "NewEnumerator0"))

(fn Reload
  (bind _returnvalue (Components|GetOwner))
  (bind _returnvalue_2 (Actor|GetComponentbyClass _returnvalue "/Game/Blueprints/Components/BP_BackPackComponent.BP_BackPackComponent_C"))
  (if (and (or (not (Variables|Configuration|GetInProcess)) (Utilities|Enum|Equal(Enum) (Variables|Configuration|GetWeaponState) "NewEnumerator2")) (Utilities|Enum|NotEqual(Enum) (Variables|Configuration|GetWeaponState) "NewEnumerator3"))
    (Variables|Configuration|SetWeaponState "NewEnumerator3")
    (Audio|Components|Audio|Play (Variables|Default|GetReloadStartSound) 0.0)
    ;[1 1 1] Reload Animation
    (Utilities|FlowControl|Sequence
      (:then_0
        (bind _asbp_character_base (Utilities|Casting|CastToBP_CharacterBase (Components|GetOwner)))
        (bind _returnvalue_3 (Animation|PlayAnimMontage _asbp_character_base (Utilities|Select :Index (Utilities|Struct|BreakSTRUCT_WeaponStats (Variables|Configuration|GetWeaponStats)) :NewEnumerator0 "/Game/AnimStarterPack/PolygoneDummy/Anim_Reload_Rifle_Hip.Anim_Reload_Rifle_Hip" :NewEnumerator1 "/Game/AnimStarterPack/PolygoneDummy/Anim_Reload_Rifle_Hip.Anim_Reload_Rifle_Hip" :NewEnumerator2 "/Game/AnimStarterPack/PolygoneDummy/Anim_Reload_Rifle_Hip.Anim_Reload_Rifle_Hip" :NewEnumerator3 "/Game/AnimStarterPack/PolygoneDummy/Anim_Reload_Rifle_Hip.Anim_Reload_Rifle_Hip" :NewEnumerator4 "/Game/AnimStarterPack/PolygoneDummy/Anim_Reload_Rifle_Hip.Anim_Reload_Rifle_Hip") 1.0 "None"))
        (LocalVariables|SetL_AnimLength _returnvalue_3)
        (if (> (LocalVariables|GetL_AnimLength) 0.0)
          (Animation|PlayAnimMontage _asbp_character_base (Utilities|Select :Index (Utilities|Struct|BreakSTRUCT_WeaponStats (Variables|Configuration|GetWeaponStats)) :NewEnumerator0 "/Game/AnimStarterPack/PolygoneDummy/Anim_Reload_Rifle_Hip.Anim_Reload_Rifle_Hip" :NewEnumerator1 "/Game/AnimStarterPack/PolygoneDummy/Anim_Reload_Rifle_Hip.Anim_Reload_Rifle_Hip" :NewEnumerator2 "/Game/AnimStarterPack/PolygoneDummy/Anim_Reload_Rifle_Hip.Anim_Reload_Rifle_Hip" :NewEnumerator3 "/Game/AnimStarterPack/PolygoneDummy/Anim_Reload_Rifle_Hip.Anim_Reload_Rifle_Hip" :NewEnumerator4 "/Game/AnimStarterPack/PolygoneDummy/Anim_Reload_Rifle_Hip.Anim_Reload_Rifle_Hip") (/ (LocalVariables|GetL_AnimLength) (Utilities|Struct|BreakSTRUCT_WeaponStats (Variables|Configuration|GetWeaponStats))) "None")))
      (:then_1
        (if (and (not (Variables|Default|GetCurrentInfinite)) (Utilities|IsValid _returnvalue_2))
          (bind _outammo (Default|UpdateAmmobyName _returnvalue_2 (- (Utilities|Struct|BreakSTRUCT_WeaponStats (Variables|Configuration|GetWeaponStats)) (Variables|Configuration|GetRoundsCurrent)) false (Variables|Configuration|GetWeaponName)))
          (Variables|Configuration|SetRoundsCurrent _outammo)
          (else
            (Variables|Configuration|SetRoundsCurrent (.RooundsMax (Utilities|Struct|BreakSTRUCT_WeaponStats (Variables|Configuration|GetWeaponStats)))))))
      (:then_2
        (if (!= (Variables|Configuration|GetRoundsCurrent) 0)
          (Utilities|Time|SetTimerbyEvent (EventDispatchers|CreateEvent :!event OnReloadDelayEnds) (.ReloadSpeed (Utilities|Struct|BreakSTRUCT_WeaponStats (Variables|Configuration|GetWeaponStats))))
          (Default|CallOnWeaponStatusChanged)
          (else
            (Variables|Configuration|SetWeaponState "NewEnumerator4")
            (Default|CallOnWeaponStatusChanged)))))))

(fn ShotFXs
  (Audio|Components|Audio|Play (Variables|Default|GetShootSound) 0.0)
  (bind _returnvalue (Game|SpawnActorfromClass "/Game/Blueprints/Weapons/Projectiles/BP_MuzzleFX.BP_MuzzleFX_C" (Transformation|GetWorldTransform (Variables|Default|GetMuzzle)) "Undefined" "MultiplyWithRoot" 0 0))
  (Transformation|AttachComponentToComponent _returnvalue (Variables|Default|GetMuzzle) "None" "SnapToTarget" "SnapToTarget" "KeepRelative" true))

(fn OnReloadDelayEnds
  (Variables|Configuration|SetWeaponState "NewEnumerator0")
  (Audio|Components|Audio|Play (Variables|Default|GetReloadEndSound) 0.0)
  (Default|CallOnWeaponStatusChanged))

(fn UpdateCurrentInfinite
  (params (InInfinit :type Boolean))
  (Variables|Default|SetCurrentInfinite InInfinit))

(fn UpdateAutoReload
  (params (InAutoReload :type Boolean))
  (Variables|Default|SetCurrentAutoReload InAutoReload))

(fn Interact
  (return false))