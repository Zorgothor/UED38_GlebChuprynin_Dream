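; NPC character Blueprint that works with BP_AIController for patrolling and combat aiming, and binds itself to a health bar widget.
; Setting a positive patrolling group switches the controller to Patrolling.
; While shooting and chasing, it interpolates the weapon muzzle toward the target, usually at its actor location and occasionally at its head bone.
; When LookAt is enabled, an AI state text label turns toward the player camera each tick.
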(event EventBeginPlay
  (|CallParentFunction)
  (bind _asw_health_bar (Utilities|Casting|CastToW_HealthBar (UserInterface|GetUserWidgetObject (Variables|Default|GetWidget))))
  (Default|UpdateCurrentCharacterforHP _asw_health_bar self))

(event EventTick
  (params (DeltaSeconds :type Float%20%28single-precision%29))
  (|CallParentFunction 0.0)
  (CallFunction|LookatPlayerCamera))

(fn ConstructionScript
  (|CallParentFunction))

(fn ActionMain
  (params (IsPressed :type Boolean))
  (|CallParentFunction IsPressed))

(fn LookatPlayerCamera
  (if (Variables|Default|GetLookAt)
    (bind _asbp_aicontroller (Utilities|Casting|CastToBP_AIController (Pawn|GetController)))
    (bind _asbp_player_character (Utilities|Casting|CastToBP_PlayerCharacter (Game|Player|GetPlayerPawn 0)))
    (Variables|Default|SetCameraLocation%20 (Transformation|GetWorldLocation (Variables|/Game/Blueprints/Character/Player/BP_PlayerCharacter.BP_PlayerCharacter_C|GetCamera _asbp_player_character)))
    (Rendering|Components|TextRender|SetText (Variables|Default|GetStateText) (Utilities|Text|FormatText "{AIState}" (Utilities|String|EnumtoString (Variables|/Game/Blueprints/Controller/BP_AIController.BP_AIController_C|GetAIState%20 _asbp_aicontroller))))
    (Transformation|SetWorldRotation (Variables|Default|GetStateText) (Math|Rotator|FindLookatRotation (Transformation|GetWorldLocation (Variables|Default|GetStateText)) (Variables|Default|GetCameraLocation%20)) false false)))

(fn UpdatePatrollingGroup
  (params (InPatrollingGroup :type Byte))
  (Variables|Default|SetPatrollingGroup InPatrollingGroup)
  (if (> (Variables|Default|GetPatrollingGroup) 0)
    (bind _asbp_aicontroller (Utilities|Casting|CastToBP_AIController (AI|GetAIController self)))
    (Default|UpdateAIState _asbp_aicontroller "NewEnumerator1")))

(fn UpdateWeaponSceneRotation
  (bind _currentweapon (Variables|Default|GetCurrentWeapon))
  (bind _muzzle (Variables|/Game/Blueprints/Weapons/BP_BaseWeapon.BP_BaseWeapon_C|GetMuzzle _currentweapon))
  (|CallParentFunction)
  (bind _currentweapon_2 (Variables|Default|GetCurrentWeapon)
    (:then
      (switch Utilities|FlowControl|Switch|SwitchonENUM_WeaponState (Variables|/Game/Blueprints/Weapons/BP_BaseWeapon.BP_BaseWeapon_C|GetWeaponState _currentweapon_2)
        (:NewEnumerator1
          (bind _asbp_aicontroller (Utilities|Casting|CastToBP_AIController (Pawn|GetController)))
          (switch Utilities|FlowControl|Switch|SwitchonENUM_AIStates (Variables|/Game/Blueprints/Controller/BP_AIController.BP_AIController_C|GetAIState%20 _asbp_aicontroller)
            (:NewEnumerator3
              (bind _targetcharacter (Variables|/Game/Blueprints/Controller/BP_AIController.BP_AIController_C|GetTargetCharacter _asbp_aicontroller)
                (:then
                  (LocalVariables|SetL_TargetLocation (Transformation|GetActorLocation _targetcharacter))
                  (if (Math|Random|RandomBoolwithWeight 0.9)
                    (Transformation|SetWorldRotation (Variables|/Game/Blueprints/Weapons/BP_BaseWeapon.BP_BaseWeapon_C|GetMuzzle (Variables|Default|GetCurrentWeapon)) (Math|Rotator|MakeRotator 0.0 (.Pitch (Math|Rotator|BreakRotator (Math|Interpolation|RInterpTo (Transformation|GetWorldRotation (Variables|/Game/Blueprints/Weapons/BP_BaseWeapon.BP_BaseWeapon_C|GetMuzzle (Variables|Default|GetCurrentWeapon))) (Math|Rotator|FindLookatRotation (Transformation|GetWorldLocation (Variables|/Game/Blueprints/Weapons/BP_BaseWeapon.BP_BaseWeapon_C|GetMuzzle (Variables|Default|GetCurrentWeapon))) (LocalVariables|GetL_TargetLocation)) (Utilities|Time|GetWorldDeltaSeconds) 1e+02))) (.Yaw (Math|Rotator|BreakRotator (Math|Interpolation|RInterpTo (Transformation|GetWorldRotation (Variables|/Game/Blueprints/Weapons/BP_BaseWeapon.BP_BaseWeapon_C|GetMuzzle (Variables|Default|GetCurrentWeapon))) (Math|Rotator|FindLookatRotation (Transformation|GetWorldLocation (Variables|/Game/Blueprints/Weapons/BP_BaseWeapon.BP_BaseWeapon_C|GetMuzzle (Variables|Default|GetCurrentWeapon))) (LocalVariables|GetL_TargetLocation)) (Utilities|Time|GetWorldDeltaSeconds) 1e+02)))) false false)
                    (else
                      (Transformation|SetWorldRotation (Variables|/Game/Blueprints/Weapons/BP_BaseWeapon.BP_BaseWeapon_C|GetMuzzle (Variables|Default|GetCurrentWeapon)) (Math|Rotator|MakeRotator 0.0 (.Pitch (Math|Rotator|BreakRotator (Math|Interpolation|RInterpTo (Transformation|GetWorldRotation _muzzle) (Math|Rotator|FindLookatRotation (Transformation|GetWorldLocation _muzzle) (.location (Transformation|GetBoneTransform (Variables|/Script/Engine.Character|GetMesh (Variables|/Game/Blueprints/Controller/BP_AIController.BP_AIController_C|GetTargetCharacter _asbp_aicontroller)) "Head" "RTS_World"))) (Utilities|Time|GetWorldDeltaSeconds) 1e+02))) (.Yaw (Math|Rotator|BreakRotator (Math|Interpolation|RInterpTo (Transformation|GetWorldRotation _muzzle) (Math|Rotator|FindLookatRotation (Transformation|GetWorldLocation _muzzle) (.location (Transformation|GetBoneTransform (Variables|/Script/Engine.Character|GetMesh (Variables|/Game/Blueprints/Controller/BP_AIController.BP_AIController_C|GetTargetCharacter _asbp_aicontroller)) "Head" "RTS_World"))) (Utilities|Time|GetWorldDeltaSeconds) 1e+02)))) false false))))
                (:else)))))))
    (:else)))