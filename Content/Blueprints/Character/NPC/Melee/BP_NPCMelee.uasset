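; BP_NPCMelee is a melee NPC that deals punch damage to friendly-faction characters through a FistHit collision component.
; When FistHit begins overlapping a BP_CharacterBase, it reads the target's CurrentFraction from BPMainStatsComponent and applies fixed BP_DamageObject damage only to Friendly ones.
; A DoOnce reset after a short delay acts as a hit cooldown shared across all targets.
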(event OnComponentBeginOverlap(FistHit)
  (params (OverlappedComponent :type Primitive%20Component%20Object%20Reference) (OtherActor :type Actor%20Object%20Reference) (OtherComp :type Primitive%20Component%20Object%20Reference) (OtherBodyIndex :type Integer) (bFromSweep :type Boolean) (SweepResult :type Hit%20Result%20Structure%20%28by%20ref%29))
  (bind _asbp_character_base (Utilities|Casting|CastToBP_CharacterBase OtherActor))
  (switch Utilities|FlowControl|Switch|SwitchonENUM_Fractions (Variables|/Game/Blueprints/Components/BP_MainStatsComponent.BP_MainStatsComponent_C|GetCurrentFraction (Variables|/Game/Blueprints/Character/BP_CharacterBase.BP_CharacterBase_C|GetBP_MainStatsComponent _asbp_character_base))
    (:NewEnumerator2
      (Utilities|FlowControl|DoOnce false :!label _label
        (:Completed
          (Game|Damage|ApplyDamage OtherActor 5.0 0 self "/Game/Blueprints/Objects/BP_DamageObject.BP_DamageObject_C")
          (Utilities|FlowControl|Delay 0.75)
          (goto _label Reset))))))

(event EventBeginPlay
  (|CallParentFunction) ; This node is disabled and will not be called.\nDrag off pins to build functionality.
)

(event Collision|EventActorBeginOverlap
  (params (OtherActor :type Actor%20Object%20Reference))
  (|CallParentFunction OtherActor) ; This node is disabled and will not be called.\nDrag off pins to build functionality.
)

(event EventTick
  (params (DeltaSeconds :type Float%20%28single-precision%29))
  (|CallParentFunction DeltaSeconds) ; This node is disabled and will not be called.\nDrag off pins to build functionality.
)

(fn ConstructionScript
  (|CallParentFunction))