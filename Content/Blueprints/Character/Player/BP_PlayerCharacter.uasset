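; Player character Blueprint that extends its parent with camera-based aiming, hit feedback and a death camera.
; Each tick it sphere-traces from the camera to steer ability and weapon muzzles at the hit point, or toward control rotation for close or missed hits.
; Stat component events drive camera shake and HP-scaled hit-feedback material parameters on damage.
; On death, the mesh ragdolls and the camera slowly turns to follow it.
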(event Custom|OnDied
  (Collision|SetCollisionProfileName (Variables|Character|GetMesh) "Ragdoll" true :!class /Script/Engine.PrimitiveComponent)
  (Physics|SetSimulatePhysics (Variables|Character|GetMesh) true)
  (Variables|Default|SetDeathCam true))

(event Custom|OnStatsUpdated
  (params (CurrentHP :type Integer) (CurrentEP :type Integer) (IsDead :type Boolean) (IsItDamage :type Boolean) (CurrentFury :type Integer))
  (if IsItDamage
    (CameraShakes|StartCameraShake (Game|GetPlayerCameraManager 0) "/Game/Blueprints/Character/Player/BP_CameraShake.BP_CameraShake_C" 1.0 "CameraLocal" "0, 0, 0")
    (Rendering|Material|SetScalarParameterValue "/Game/Art/Materials/Collection/MPC_HitFeedback.MPC_HitFeedback" "Radius" (Math|Float|MapRangeClamped (Math|Conversions|ToFloat(Integer) (Variables|/Game/Blueprints/Components/BP_MainStatsComponent.BP_MainStatsComponent_C|GetCurrentHP (Variables|Default|GetBP_MainStatsComponent))) 0.0 (Math|Conversions|ToFloat(Integer) (.MaxHP (Utilities|Struct|BreakSTRUCT_MainStats (Variables|/Game/Blueprints/Components/BP_MainStatsComponent.BP_MainStatsComponent_C|GetMainStatsStructure (Variables|Default|GetBP_MainStatsComponent))))) 1.0 2.0) :!class /Script/Engine.KismetMaterialLibrary)
    (Rendering|Material|SetScalarParameterValue "/Game/Art/Materials/Collection/MPC_HitFeedback.MPC_HitFeedback" "Density" (Math|Float|MapRangeClamped (Math|Conversions|ToFloat(Integer) (Variables|/Game/Blueprints/Components/BP_MainStatsComponent.BP_MainStatsComponent_C|GetCurrentHP (Variables|Default|GetBP_MainStatsComponent))) 0.0 (Math|Conversions|ToFloat(Integer) (.MaxHP (Utilities|Struct|BreakSTRUCT_MainStats (Variables|/Game/Blueprints/Components/BP_MainStatsComponent.BP_MainStatsComponent_C|GetMainStatsStructure (Variables|Default|GetBP_MainStatsComponent))))) 2.0 3.0) :!class /Script/Engine.KismetMaterialLibrary)))

(event EventBeginPlay
  (|CallParentFunction)
  (EventDispatchers|BindEventtoOnStatsUpdated (Variables|Default|GetBP_MainStatsComponent) (delegate Custom|OnStatsUpdated))
  (EventDispatchers|BindEventtoOnDead (Variables|Default|GetBP_MainStatsComponent) (delegate Custom|OnDied)))

(event EventTick
  (params (DeltaSeconds :type Float%20%28single-precision%29))
  (CallFunction|UpdateAbilityMuzzleRotation)
  (CallFunction|UpdateWeaponSceneRotation)
  (if (Variables|Default|GetDeathCam)
    (Transformation|SetWorldRotation (Variables|Default|GetCamera) (Math|Interpolation|RInterpTo (Transformation|GetWorldRotation (Variables|Default|GetCamera)) (Math|Rotator|FindLookatRotation (Transformation|GetWorldLocation (Variables|Default|GetCamera)) (Transformation|GetWorldLocation (Variables|Character|GetMesh))) (Utilities|Time|GetWorldDeltaSeconds) 1.0) false false)))

(fn ConstructionScript
  (|CallParentFunction))

(fn ActionMain
  (params (IsPressed :type Boolean))
  (|CallParentFunction IsPressed))

(fn UpdateWeaponSceneRotation
  (bind _camera (Variables|Default|GetCamera))
  (bind _returnvalue (Transformation|GetWorldLocation _camera))
  (|CallParentFunction)
  (bind _currentweapon (Variables|Default|GetCurrentWeapon)
    (:then
      (LocalVariables|SetL_WeaponMuzzle (Variables|/Game/Blueprints/Weapons/BP_BaseWeapon.BP_BaseWeapon_C|GetMuzzle _currentweapon))
      (switch Utilities|FlowControl|Switch|SwitchonENUM_WeaponState (Variables|/Game/Blueprints/Weapons/BP_BaseWeapon.BP_BaseWeapon_C|GetWeaponState (Variables|Default|GetCurrentWeapon))
        (:NewEnumerator0
          _)
        (:NewEnumerator1
          _))
      (bind (_outhit _returnvalue_2) (Collision|SphereTraceByChannel _returnvalue (+ _returnvalue (* (Math|Vector|GetForwardVector _camera) 10000)) 0.1 "TraceTypeQuery2" true (Utilities|Array|MakeArray self (Variables|Default|GetCurrentWeapon)) "None" true "(R=1.000000,G=0.000000,B=0.000000,A=1.000000)" "(R=0.000000,G=1.000000,B=0.000000,A=1.000000)" 0.0))
      (if _returnvalue_2
        (if (> (.Distance (Collision|BreakHitResult _outhit)) 2.5e+02)
          (Transformation|SetWorldRotation (LocalVariables|GetL_WeaponMuzzle) (Math|Interpolation|RInterpTo (Transformation|GetWorldRotation (LocalVariables|GetL_WeaponMuzzle)) (Math|Rotator|FindLookatRotation (Transformation|GetWorldLocation (LocalVariables|GetL_WeaponMuzzle)) (.Location (Collision|BreakHitResult _outhit))) (Utilities|Time|GetWorldDeltaSeconds) 1e+02) false false)
          (else
            (Transformation|SetWorldRotation (LocalVariables|GetL_WeaponMuzzle) (Math|Interpolation|RInterpTo (Transformation|GetWorldRotation (LocalVariables|GetL_WeaponMuzzle)) (Pawn|GetControlRotation :!class /Script/Engine.Pawn) (Utilities|Time|GetWorldDeltaSeconds) 1e+02) false false :!label _label)))
        (else
          (goto _label))))
    (:else)))

(fn UpdateAbilityMuzzleRotation
  (bind _camera (Variables|Default|GetCamera))
  (bind _returnvalue (Transformation|GetWorldLocation _camera))
  (bind (_outhit _returnvalue_2) (Collision|SphereTraceByChannel _returnvalue (+ _returnvalue (* (Math|Vector|GetForwardVector _camera) 10000)) 0.1 "TraceTypeQuery2" true (Utilities|Array|MakeArray self (Variables|Default|GetCurrentWeapon)) "None" true "(R=1.000000,G=0.000000,B=0.000000,A=1.000000)" "(R=0.000000,G=1.000000,B=0.000000,A=1.000000)" 0.0))
  (if _returnvalue_2
    (if (> (.Distance (Collision|BreakHitResult _outhit)) 2.5e+02)
      (Transformation|SetWorldRotation (Variables|Default|GetAbilityMuzzle) (Math|Interpolation|RInterpTo (Transformation|GetWorldRotation (Variables|Default|GetAbilityMuzzle)) (Math|Rotator|FindLookatRotation (Transformation|GetWorldLocation (Variables|Default|GetAbilityMuzzle)) (.Location (Collision|BreakHitResult _outhit))) (Utilities|Time|GetWorldDeltaSeconds) 1e+02) false false)
      (else
        (Transformation|SetWorldRotation (Variables|Default|GetAbilityMuzzle) (Math|Interpolation|RInterpTo (Transformation|GetWorldRotation (Variables|Default|GetAbilityMuzzle)) (Pawn|GetControlRotation :!class /Script/Engine.Pawn) (Utilities|Time|GetWorldDeltaSeconds) 1e+02) false false :!label _label)))
    (else
      (goto _label))))